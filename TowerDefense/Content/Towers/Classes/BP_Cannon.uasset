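; BP_Cannon is a cannon tower class for a tower defense game, with almost no active logic of its own.
; On BeginPlay it casts and caches the tower defense game mode.
; The tower mesh click event is empty, and the disconnected nodes that would select the tower and show the overlay's upgrade panel never run.
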(event OnClicked(TowerMesh)
  (params (TouchedComponent :type Primitive%20Component%20Object%20Reference) (ButtonPressed :type Key%20Structure)))

(event EventBeginPlay
  (bind _asbp_tower_defense_game_mode (Utilities|Casting|CastToBP_TowerDefenseGameMode (Game|GetGameMode)))
  (Variables|Default|SetTowerDefenseGameMode _asbp_tower_defense_game_mode))

(fn ConstructionScript)