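; BP_Enemy_4 is an enemy actor that travels along the level's track spline.
; On BeginPlay it takes the first BP_Track found in the world and starts a timeline whose play rate is the inverse of Duration.
; Each timeline update lerps Alpha over the spline length and sets the enemy's world location and rotation to that point on UsefulSpline.
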(event Custom|MoveEnemyOnSpline
  (Components|Timeline|SetPlayRate (Variables|Default|GetMoveAlongSpline) (/ 1.0 (Variables|Default|GetDuration)))
  (bind _alpha (Timeline|MoveAlongSpline Play)
    (:Update
      (bind _output_get (Variables|Default|SetAlpha _alpha))
      (Transformation|SetActorLocationAndRotation (Spline|GetLocationatDistanceAlongSpline (Variables|/Game/Pathfinding/BP_Track.BP_Track_C|GetUsefulSpline (Variables|Default|GetSpline)) (Math|Float|Lerp 0.0 (Spline|GetSplineLength (Variables|/Game/Pathfinding/BP_Track.BP_Track_C|GetUsefulSpline (Variables|Default|GetSpline))) _output_get) "World") (Spline|GetRotationatDistanceAlongSpline (Variables|/Game/Pathfinding/BP_Track.BP_Track_C|GetUsefulSpline (Variables|Default|GetSpline)) (Math|Float|Lerp 0.0 (Spline|GetSplineLength (Variables|/Game/Pathfinding/BP_Track.BP_Track_C|GetUsefulSpline (Variables|Default|GetSpline))) _output_get) "World")))))

(event EventBeginPlay
  (bind _outactors (Actor|GetAllActorsOfClass "/Game/Pathfinding/BP_Track.BP_Track_C"))
  (Variables|Default|SetSpline (Utilities|Array|Get(acopy) _outactors))
  (CallFunction|MoveEnemyonSpline))

(fn ConstructionScript)